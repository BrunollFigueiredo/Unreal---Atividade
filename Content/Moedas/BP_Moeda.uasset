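; BP_Moeda is a coin pickup that the player pawn collects by overlapping it.
; A one-shot flag guards collection, then the coin's value, at least one, is added to the running total in the BP_ContadorMoedas Game Instance and printed.
; The same amount is passed to a bp_http actor found in the level to save it, then the coin destroys itself.
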(event Collision|EventActorBeginOverlap
  (params (OtherActor :type Actor%20Object%20Reference))
  (if (== OtherActor (Game|Player|GetPlayerPawn 0))
    (if (not (Variables|Default|GetJaColetada))
      (bind _asbp_contador_moedas (Utilities|Casting|CastToBP_ContadorMoedas (Game|GetGameInstance)))
      (Variables|Default|SetJaColetada true)
      (bind _output_get (Variables|/Game/Moedas/BP_ContadorMoedas.BP_ContadorMoedas_C|SetTotalMoedas _asbp_contador_moedas (+ (Variables|/Game/Moedas/BP_ContadorMoedas.BP_ContadorMoedas_C|GetTotalMoedas _asbp_contador_moedas) (Math|Integer|Max(Integer) (Variables|Default|GetValorMoeda) 1))))
      (Development|PrintString (Utilities|String|Append "Moedas: " (Utilities|String|ToString(Integer) _output_get)) true true "(R=1.0,G=0.8,B=0.05,A=1.0)" 3.0 "ContadorMoedas")
      (bind _returnvalue (Actor|GetActorOfClass "/Game/bp_http.bp_http_C"))
      (bind _asbp_http (Utilities|Casting|CastTobp_http _returnvalue)
        (:then
          (Default|SalvarMoedasColetadas _asbp_http (Math|Integer|Max(Integer) (Variables|Default|GetValorMoeda) 1)))
        (:CastFailed
          _))
      (Actor|DestroyActor))))

(event EventBeginPlay)

(event EventTick
  (params (DeltaSeconds :type Float%20%28single-precision%29)))

(fn ConstructionScript)