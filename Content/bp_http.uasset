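; Actor Blueprint that reads, inserts and deletes player records through a REST API.
; BeginPlay, the G key or SelectBD fetches the player by PlayerId and stores its "nome" in NomePlayer.
; The I key or InsertBD posts NomePlayer as struct-built JSON and saves the returned insertId as PlayerId.
; The Delete key or DeleteBD removes the player with that ID, and request results are printed on screen.
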(event Custom|SelectBD
  ;[0.1 0.17 0.23] Select BD | BeginPlay / G | GET /player/{PlayerId} -> nome -> NomePlayer
  (bind _result_body (|HttpRequest (Utilities|String|Append (Utilities|String|Append (Variables|Default|GetApiBaseUrl) "/player/") (Utilities|String|ToString(Integer) (Variables|Default|GetPlayerId))) "Get" (|MakeRequestHeader "Json"))
    (:On%20Success
      (bind (_outjsonobject _returnvalue) (Class|JsonBlueprintFunctionLibrary|FromString _result_body))
      (if _returnvalue
        (bind (_outvalue _returnvalue_2) (Class|JsonBlueprintFunctionLibrary|GetField _outjsonobject "nome"))
        (if _returnvalue_2
          (bind _output_get (Variables|Default|SetNomePlayer _outvalue))
          (Development|PrintString _output_get true true "(R=0.000000,G=0.660000,B=1.000000,A=1.000000)" 6.0)
          (else
            (Development|PrintString _result_body true true "(R=0.000000,G=0.660000,B=1.000000,A=1.000000)" 6.0)))
        (else
          (Development|PrintString "GET: JSON invalido" true true "(R=0.000000,G=0.660000,B=1.000000,A=1.000000)" 6.0))))
    (:On%20Error
      (Development|PrintString _result_body true true "(R=0.000000,G=0.660000,B=1.000000,A=1.000000)" 6.0))))

(event Custom|InsertBD
  ;[0.1 0.17 0.23] Insert BD | I | NomePlayer -> Struct Player (nome string) -> JSON -> POST | guarda insertId
  (bind (_outjsonstring _returnvalue) (Class|JsonBlueprintFunctionLibrary|StructtoJsonString (Utilities|Struct|MakeStruct_PlayerAPI false (Variables|Default|GetNomePlayer))))
  (if _returnvalue
    (bind _result_body (|HttpRequest (Utilities|String|Append (Variables|Default|GetApiBaseUrl) "/player/insertPlayer") "Post" (|MakeRequestHeader "Json") _outjsonstring)
      (:On%20Success
        (bind _outjsonobject (Class|JsonBlueprintFunctionLibrary|FromString _result_body))
        (bind _outvalue (Class|JsonBlueprintFunctionLibrary|GetField _outjsonobject "success"))
        (if _outvalue
          (bind _outvalue_2 (Class|JsonBlueprintFunctionLibrary|GetField _outjsonobject "insertId"))
          (Variables|Default|SetPlayerId _outvalue_2)
          (Development|PrintString _result_body true true "(R=0.000000,G=0.660000,B=1.000000,A=1.000000)" 6.0)
          (else
            (Development|PrintString _result_body true true "(R=0.000000,G=0.660000,B=1.000000,A=1.000000)" 6.0))))
      (:On%20Error
        (Development|PrintString _result_body true true "(R=0.000000,G=0.660000,B=1.000000,A=1.000000)" 6.0)))
    (else
      (Development|PrintString "Falha ao converter Struct Player para JSON" true true "(R=0.000000,G=0.660000,B=1.000000,A=1.000000)" 6.0))))

(event Custom|DeleteBD
  ;[0.1 0.17 0.23] Delete BD | Delete | DELETE /player/deletePlayer/{PlayerId} | exclusao somente por acao explicita
  (bind _result_body (|HttpRequest (Utilities|String|Append (Utilities|String|Append (Variables|Default|GetApiBaseUrl) "/player/deletePlayer/") (Utilities|String|ToString(Integer) (Variables|Default|GetPlayerId))) "Delete" (|MakeRequestHeader "Json") (Utilities|String|MakeLiteralString "{}"))
    (:On%20Success
      (bind _outjsonobject (Class|JsonBlueprintFunctionLibrary|FromString _result_body))
      (bind _outvalue (Class|JsonBlueprintFunctionLibrary|GetField _outjsonobject "success"))
      (if _outvalue
        (Development|PrintString _result_body true true "(R=0.000000,G=0.660000,B=1.000000,A=1.000000)" 6.0)
        (else
          (Development|PrintString _result_body true true "(R=0.000000,G=0.660000,B=1.000000,A=1.000000)" 6.0))))
    (:On%20Error
      (Development|PrintString _result_body true true "(R=0.000000,G=0.660000,B=1.000000,A=1.000000)" 6.0))))

(event EventBeginPlay
  ;[0.1 0.17 0.23] Select BD | BeginPlay / G | GET /player/{PlayerId} -> nome -> NomePlayer
  (bind _result_body (|HttpRequest (Utilities|String|Append (Utilities|String|Append (Variables|Default|GetApiBaseUrl) "/player/") (Utilities|String|ToString(Integer) (Variables|Default|GetPlayerId))) "Get" (|MakeRequestHeader "Json"))
    (:On%20Success
      (bind (_outjsonobject _returnvalue) (Class|JsonBlueprintFunctionLibrary|FromString _result_body))
      (if _returnvalue
        (bind (_outvalue _returnvalue_2) (Class|JsonBlueprintFunctionLibrary|GetField _outjsonobject "nome"))
        (if _returnvalue_2
          (bind _output_get (Variables|Default|SetNomePlayer _outvalue))
          (Development|PrintString _output_get true true "(R=0.000000,G=0.660000,B=1.000000,A=1.000000)" 6.0)
          (else
            (Development|PrintString _result_body true true "(R=0.000000,G=0.660000,B=1.000000,A=1.000000)" 6.0)))
        (else
          (Development|PrintString "GET: JSON invalido" true true "(R=0.000000,G=0.660000,B=1.000000,A=1.000000)" 6.0))))
    (:On%20Error
      (Development|PrintString _result_body true true "(R=0.000000,G=0.660000,B=1.000000,A=1.000000)" 6.0))))

(event Input|KeyboardEvents|G
  (params (Key :type Key%20Structure))
  (:Pressed
    ;[0.1 0.17 0.23] Select BD | BeginPlay / G | GET /player/{PlayerId} -> nome -> NomePlayer
    (bind _result_body (|HttpRequest (Utilities|String|Append (Utilities|String|Append (Variables|Default|GetApiBaseUrl) "/player/") (Utilities|String|ToString(Integer) (Variables|Default|GetPlayerId))) "Get" (|MakeRequestHeader "Json"))
      (:On%20Success
        (bind (_outjsonobject _returnvalue) (Class|JsonBlueprintFunctionLibrary|FromString _result_body))
        (if _returnvalue
          (bind (_outvalue _returnvalue_2) (Class|JsonBlueprintFunctionLibrary|GetField _outjsonobject "nome"))
          (if _returnvalue_2
            (bind _output_get (Variables|Default|SetNomePlayer _outvalue))
            (Development|PrintString _output_get true true "(R=0.000000,G=0.660000,B=1.000000,A=1.000000)" 6.0)
            (else
              (Development|PrintString _result_body true true "(R=0.000000,G=0.660000,B=1.000000,A=1.000000)" 6.0)))
          (else
            (Development|PrintString "GET: JSON invalido" true true "(R=0.000000,G=0.660000,B=1.000000,A=1.000000)" 6.0))))
      (:On%20Error
        (Development|PrintString _result_body true true "(R=0.000000,G=0.660000,B=1.000000,A=1.000000)" 6.0)))))

(event Input|KeyboardEvents|I
  (params (Key :type Key%20Structure))
  (:Pressed
    ;[0.1 0.17 0.23] Insert BD | I | NomePlayer -> Struct Player (nome string) -> JSON -> POST | guarda insertId
    (bind (_outjsonstring _returnvalue) (Class|JsonBlueprintFunctionLibrary|StructtoJsonString (Utilities|Struct|MakeStruct_PlayerAPI false (Variables|Default|GetNomePlayer))))
    (if _returnvalue
      (bind _result_body (|HttpRequest (Utilities|String|Append (Variables|Default|GetApiBaseUrl) "/player/insertPlayer") "Post" (|MakeRequestHeader "Json") _outjsonstring)
        (:On%20Success
          (bind _outjsonobject (Class|JsonBlueprintFunctionLibrary|FromString _result_body))
          (bind _outvalue (Class|JsonBlueprintFunctionLibrary|GetField _outjsonobject "success"))
          (if _outvalue
            (bind _outvalue_2 (Class|JsonBlueprintFunctionLibrary|GetField _outjsonobject "insertId"))
            (Variables|Default|SetPlayerId _outvalue_2)
            (Development|PrintString _result_body true true "(R=0.000000,G=0.660000,B=1.000000,A=1.000000)" 6.0)
            (else
              (Development|PrintString _result_body true true "(R=0.000000,G=0.660000,B=1.000000,A=1.000000)" 6.0))))
        (:On%20Error
          (Development|PrintString _result_body true true "(R=0.000000,G=0.660000,B=1.000000,A=1.000000)" 6.0)))
      (else
        (Development|PrintString "Falha ao converter Struct Player para JSON" true true "(R=0.000000,G=0.660000,B=1.000000,A=1.000000)" 6.0)))))

(event Input|KeyboardEvents|Delete
  (params (Key :type Key%20Structure))
  (:Pressed
    ;[0.1 0.17 0.23] Delete BD | Delete | DELETE /player/deletePlayer/{PlayerId} | exclusao somente por acao explicita
    (bind _result_body (|HttpRequest (Utilities|String|Append (Utilities|String|Append (Variables|Default|GetApiBaseUrl) "/player/deletePlayer/") (Utilities|String|ToString(Integer) (Variables|Default|GetPlayerId))) "Delete" (|MakeRequestHeader "Json") (Utilities|String|MakeLiteralString "{}"))
      (:On%20Success
        (bind _outjsonobject (Class|JsonBlueprintFunctionLibrary|FromString _result_body))
        (bind _outvalue (Class|JsonBlueprintFunctionLibrary|GetField _outjsonobject "success"))
        (if _outvalue
          (Development|PrintString _result_body true true "(R=0.000000,G=0.660000,B=1.000000,A=1.000000)" 6.0)
          (else
            (Development|PrintString _result_body true true "(R=0.000000,G=0.660000,B=1.000000,A=1.000000)" 6.0))))
      (:On%20Error
        (Development|PrintString _result_body true true "(R=0.000000,G=0.660000,B=1.000000,A=1.000000)" 6.0)))))

(fn ConstructionScript)